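; End-of-level checkpoint actor that advances the game to the next level when stepped on with all Cubes dead.
; Its construction script offsets it by Subtraction and calls Spawn, a self-calling delayed event that lerps it back into place.
; SteppedOn works once, setting itself as every PolarBearCharacter's checkpoint and spawning a row of Logs from the game mode's current position.
; It then moves the main camera up and has GamemodeForNow start the next level.
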(event Custom|Spawn
  (bind _supposedlocation (Variables|Default|GetSupposedLocation))
  (Utilities|FlowControl|Delay 0.01)
  (Transformation|SetActorLocation (Math|Vector|Lerp(Vector) (- _supposedlocation (Variables|Default|GetSubtraction)) _supposedlocation (Variables|Default|GetAlpha)) false false)
  (bind _output_get (Variables|Default|SetAlpha (+ (Variables|Default|GetAlpha) 0.02)))
  (if (< _output_get 1.0)
    (CallFunction|Spawn)
    (else
      (Transformation|SetActorLocation (Variables|Default|GetSupposedLocation) false false))))

(event EventBeginPlay)

(event Collision|EventActorBeginOverlap
  (params (OtherActor :type Actor%20Object%20Reference)))

(event EventTick
  (params (DeltaSeconds :type Float%20%28single-precision%29)))

(fn ConstructionScript
  (bind _output_get (Variables|Default|SetSupposedLocation (Transformation|GetActorLocation)))
  (Transformation|SetActorLocation (- _output_get (Variables|Default|GetSubtraction)) false false)
  (CallFunction|Spawn))

(fn Steppedon
  (if (not (Variables|Default|GetUsed))
    (bind _outactors (Actor|GetAllActorsOfClass "/Game/Blueprints/Cube.Cube_C"))
    ;[1 1 1] Make sure any still *alive* are dying
    (for _array_element _outactors
      (if (not (Variables|/Game/Blueprints/Cube.Cube_C|Getdead _array_element))
        (Variables|Default|SetAllDead false)))
    (if (or (Variables|Default|GetAllDead) (== (Utilities|Array|Length _outactors) 0))
      (Utilities|FlowControl|Sequence
        (:then_0
          (bind _outactors_2 (Actor|GetAllActorsOfClass "/Game/Blueprints/PolarBearCharacter.PolarBearCharacter_C"))
          (for _array_element_2 _outactors_2
            (bind _aspolar_bear_character (Utilities|Casting|CastToPolarBearCharacter _array_element_2))
            (Variables|/Game/Blueprints/PolarBearCharacter.PolarBearCharacter_C|SetCheckpoint _aspolar_bear_character self)))
        (:then_1
          (Variables|Default|SetUsed true)
          (bind _asgamemode_for_now (Utilities|Casting|CastToGamemodeForNow (Game|GetGameMode)))
          (Variables|/Game/Blueprints/GamemodeForNow.GamemodeForNow_C|SetOldPosition _asgamemode_for_now (Variables|/Game/Blueprints/GamemodeForNow.GamemodeForNow_C|GetCurrentPosition _asgamemode_for_now))
          (for _index (range 0 3)
            (bind _output_get (Variables|/Game/Blueprints/GamemodeForNow.GamemodeForNow_C|SetCurrentPosition _asgamemode_for_now (+ (Variables|/Game/Blueprints/GamemodeForNow.GamemodeForNow_C|GetCurrentPosition _asgamemode_for_now) "100.000000,0.000000, 0")))
            (Game|SpawnActorfromClass "/Game/Blueprints/Log.Log_C" (Math|Transform|MakeTransform _output_get "0, 0, 0" "1,1,1") "Undefined" 0 _index 0))
          (Variables|/Game/Blueprints/GamemodeForNow.GamemodeForNow_C|SetCurrentPosition _asgamemode_for_now (+ (Variables|/Game/Blueprints/GamemodeForNow.GamemodeForNow_C|GetCurrentPosition _asgamemode_for_now) "100.000000,0.000000, 0"))
          (bind _outactors_3 (Actor|GetAllActorsOfClass "/Game/Blueprints/MainCameraController.MainCameraController_C"))
          (Default|MoveUp (Utilities|Array|Get(acopy) _outactors_3) self)
          (bind _asgamemode_for_now_2 (Utilities|Casting|CastToGamemodeForNow (Game|GetGameMode)))
          (bind _levelname (Default|SetNextLevel _asgamemode_for_now_2))
          (Default|StartLevel _asgamemode_for_now_2 _levelname false))))))