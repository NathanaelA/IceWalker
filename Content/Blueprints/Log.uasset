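; Log is a moving platform actor that slides back and forth along the world Y axis and carries a character that steps on it.
; The construction script randomizes direction and speed and picks the starting end; Tick moves it a fixed step per frame, without delta time, reversing past fixed bounds.
; SteppedOn stores a signed distance offset, which Tick uses to lock the character's Y to the log; nothing here clears that attachment.
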(event EventBeginPlay)

(event Collision|EventActorBeginOverlap
  (params (OtherActor :type Actor%20Object%20Reference)))

(event EventTick
  (params (DeltaSeconds :type Float%20%28single-precision%29))
  (bind _returnvalue (Transformation|GetActorLocation))
  (bind _character (Variables|Default|GetCharacter))
  (bind _returnvalue_2 (Transformation|GetActorLocation _character))
  (if (Variables|Default|GetForward)
    (Variables|Default|SetY (+ (Variables|Default|GetY) (Variables|Default|GetSpeed)))
    (else
      (Variables|Default|SetY (- (Variables|Default|GetY) (Variables|Default|GetSpeed)))))
  (Transformation|SetActorLocation (Math|Vector|MakeVector (.x _returnvalue) (Variables|Default|GetY) (.z _returnvalue)) false false)
  (if (< (Variables|Default|GetY) -5e+02)
    (Variables|Default|SetForward true)
    (elif (> (Variables|Default|GetY) 5e+02)
      (Variables|Default|SetForward false)))
  (if (Variables|Default|GetPlayerOn)
    (Transformation|SetActorLocation _character (Math|Vector|MakeVector (.x _returnvalue_2) (+ (.y (Transformation|GetActorLocation)) (Variables|Default|GetPlayerYOffset)) (.z _returnvalue_2)) false false)))

(fn ConstructionScript
  (bind _output_get (Variables|Default|SetForward (Math|Random|RandomBool)))
  (if _output_get
    (Variables|Default|SetY -1e+03)
    (else
      (Variables|Default|SetY 1e+03)))
  (Variables|Default|SetSpeed (Math|Random|RandomFloatinRange 5.0 2e+01)))

(fn Steppedon
  (params (Character :type Actor%20Object%20Reference))
  (bind _self self)
  (bind _returnvalue (Transformation|GetDistanceTo Character _self))
  (Variables|Default|SetCharacter Character)
  (Variables|Default|SetPlayerOn true)
  (if (> (Variables|Default|GetY) (.y (Transformation|GetActorLocation Character)))
    (Variables|Default|SetPlayerYOffset (- _returnvalue (* _returnvalue 2.0)))
    (else
      (Variables|Default|SetPlayerYOffset _returnvalue))))