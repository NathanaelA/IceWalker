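; IceWalkerPlayerController is a player controller Blueprint that creates the player's polar bear character and drives its movement.
; Its Start event clears all widgets, spawns a PolarBearCharacter, stores it as Char and calls Animate on it.
; The Left, Right, Up and Down input actions call the matching move functions on that stored reference on press, with no possession step in the graph.
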(event Custom|Start
  (Viewport|RemoveAllWidgets)
  (bind _returnvalue (Game|SpawnActorfromClass "/Game/Blueprints/PolarBearCharacter.PolarBearCharacter_C" (Math|Transform|MakeTransform "0, 0, 0" "0, 0, 0" "1,1,1") "Undefined" 0 true 0))
  (bind _output_get (Variables|Default|SetChar _returnvalue))
  (Default|Animate _output_get))

(event EventBeginPlay)

(event Input|ActionEvents|InputActionLeft
  (params (Key :type Key%20Structure))
  (:Pressed
    (Default|MoveLeft (Variables|Default|GetChar))))

(event Input|ActionEvents|InputActionRight
  (params (Key :type Key%20Structure))
  (:Pressed
    (Default|MoveRight (Variables|Default|GetChar))))

(event Input|ActionEvents|InputActionUp
  (params (Key :type Key%20Structure))
  (:Pressed
    (Default|MoveUp (Variables|Default|GetChar))))

(event Input|ActionEvents|InputActionDown
  (params (Key :type Key%20Structure))
  (:Pressed
    (Default|MoveDown (Variables|Default|GetChar))))

(fn ConstructionScript)