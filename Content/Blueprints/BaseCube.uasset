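; BaseCube is a base tile actor that rises into place when spawned and sinks away when destroyed, with stub SteppedOn hooks returning false.
; The construction script lowers it, then Spawn lerps it up through delayed self-calls, or snaps under InstantTiles.
; Destroy disables collision and recursively sinks it until deletion, but hands WhiteIce to GoThroughMaterials unless instant.
; Keep pins the tile in place and blocks normal sinking.
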(event Custom|Destroy
  (params (Instant :type Boolean))
  (bind _returnvalue (Transformation|GetActorLocation))
  (bind _returnvalue_2 (- _returnvalue "0, 0,2.000000"))
  (bind _aswhite_ice (Utilities|Casting|CastToWhiteIce self)
    (:then
      (if Instant
        (Actor|DestroyActor)
        (else
          (bind _asgamemode_for_now (Utilities|Casting|CastToGamemodeForNow (Game|GetGameMode))
            (:then
              (Default|GoThroughMaterials _aswhite_ice (Utilities|Array|Length (Variables|/Game/Blueprints/GamemodeForNow.GamemodeForNow_C|GetWhiteIceMaterials _asgamemode_for_now))))
            (:CastFailed
              (if (not (Variables|Default|GetkeepForever)) :!label _label
                (Variables|Default|Setdead true)
                (Collision|SetCollisionResponsetoAllChannels (Variables|Default|GetCube) "ECR_Ignore")
                (Utilities|FlowControl|Delay 0.05)
                (if Instant
                  (Actor|DestroyActor)
                  (else
                    (Transformation|SetActorLocation _returnvalue_2 false false)
                    (CallFunction|Destroy (< (.Z (Math|Vector|BreakVector _returnvalue_2)) -4e+02))))))))))
    (:CastFailed
      (goto _label))))

(event Custom|Spawn
  (bind _supposedlocation (Variables|Default|GetSupposedLocation))
  (bind _asgamemode_for_now (Utilities|Casting|CastToGamemodeForNow (Game|GetGameMode)))
  (if (Variables|/Game/Blueprints/GamemodeForNow.GamemodeForNow_C|GetinstantTiles _asgamemode_for_now)
    (Transformation|SetActorLocation (Variables|Default|GetSupposedLocation) false false :!label _label)
    (else
      (Utilities|FlowControl|Delay 0.01)
      (Transformation|SetActorLocation (Math|Vector|Lerp(Vector) (- _supposedlocation (Variables|Default|GetSubtraction)) _supposedlocation (Variables|Default|GetAlpha)) false false)
      (bind _output_get (Variables|Default|SetAlpha (+ (Variables|Default|GetAlpha) (Variables|Default|GetSpawnSpeed))))
      (if (< _output_get 1.0)
        (CallFunction|Spawn)
        (else
          (goto _label))))))

(event EventBeginPlay)

(event Collision|EventActorBeginOverlap
  (params (OtherActor :type Actor%20Object%20Reference)))

(event EventTick
  (params (DeltaSeconds :type Float%20%28single-precision%29)))

(fn ConstructionScript
  (if (not (Variables|Default|GetkeepForever))
    (bind _output_get (Variables|Default|SetSupposedLocation (Transformation|GetActorLocation)))
    (Transformation|SetActorLocation (- _output_get (Variables|Default|GetSubtraction)) false false)
    (CallFunction|Spawn)))

(fn Steppedon
  (return false))

(fn AfterSteppedon
  (params (Update :type Boolean))
  (return false))

(fn Keep
  (Variables|Default|SetkeepForever true)
  (Transformation|SetActorLocation (Variables|Default|GetSupposedLocation) false false))