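; Controls the main game camera, giving it a fixed starting view and sliding it along X to follow a given actor.
; MoveUp eases the camera to a fixed X offset from the actor using a timeline lerp, keeping Y, Z and rotation.
; UpdateCameras, run on construction, Start and each move, caches a scene CameraActor and destroys any found near the world origin.
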(event Custom|MoveUp
  (params (Actor :type Actor%20Object%20Reference))
  (bind _camera (Variables|Default|GetCamera))
  (CallFunction|UpdateCameras)
  (bind _output_get (Variables|Default|SetOldLocation (Transformation|GetActorLocation (Variables|Default|GetCamera))))
  (Variables|Default|SetNewLocation (Math|Vector|MakeVector (- (.x (Transformation|GetActorLocation Actor)) 225.0) (.Y (Math|Vector|BreakVector _output_get)) (.Z (Math|Vector|BreakVector _output_get))))
  (bind _alpha (Timeline|CameraDistance Play)
    (:Update
      (Transformation|SetActorTransform _camera (Math|Transform|MakeTransform (Math|Vector|Lerp(Vector) (Variables|Default|GetOldLocation) (Variables|Default|GetNewLocation) _alpha) (Transformation|GetActorRotation _camera) "1,1,1")))))

(fn ConstructionScript
  (CallFunction|UpdateCameras))

(fn Start
  (CallFunction|UpdateCameras)
  (Transformation|SetActorTransform (Variables|Default|GetCamera) (Math|Transform|MakeTransform "-925.000000,150.000000,895.000000" "-50.000000,340.000000,0.000000" "1,1,1")))

(fn UpdateCameras
  (bind _outactors (Actor|GetAllActorsOfClass "/Script/Engine.CameraActor"))
  (for _array_element _outactors
    (if (Math|Vector|Equal(Vector) (Transformation|GetActorLocation _array_element) "0, 0, 0" 1.0)
      (Actor|DestroyActor _array_element)
      (else
        (Variables|Default|SetCamera _array_element)))))