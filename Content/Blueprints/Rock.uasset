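; Rock actor that animates into its placed position on spawn and sinks away when destroyed.
; The construction script records the placed location, offsets the actor by Subtraction and calls Spawn, which lerps it back.
; Destroy sets Dead, disables Cube collision responses, then either removes the actor instantly or lowers it until below a Z threshold.
; Both animations use self-calling events with short Delays instead of Tick or Timelines.
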(event Custom|Destroy
  (params (instant :type Boolean))
  (bind _returnvalue (Transformation|GetActorLocation))
  (bind _returnvalue_2 (- _returnvalue "0, 0,2.000000"))
  (Variables|Default|Setdead true)
  (Collision|SetCollisionResponsetoAllChannels (Variables|Default|GetCube) "ECR_Ignore")
  (Utilities|FlowControl|Delay 0.005)
  (if instant
    (Actor|DestroyActor)
    (else
      (Transformation|SetActorLocation _returnvalue_2 false false)
      (CallFunction|Destroy (< (.Z (Math|Vector|BreakVector _returnvalue_2)) -4e+02)))))

(event Custom|Spawn
  (bind _supposedlocation (Variables|Default|GetSupposedLocation))
  (Utilities|FlowControl|Delay 0.01)
  (Transformation|SetActorLocation (Math|Vector|Lerp(Vector) (- _supposedlocation (Variables|Default|GetSubtraction)) _supposedlocation (Variables|Default|GetAlpha)) false false)
  (bind _output_get (Variables|Default|SetAlpha (+ (Variables|Default|GetAlpha) 0.1)))
  (if (< _output_get 1.0)
    (CallFunction|Spawn)
    (else
      (Transformation|SetActorLocation (Variables|Default|GetSupposedLocation) false false))))

(fn ConstructionScript
  (bind _output_get (Variables|Default|SetSupposedLocation (Transformation|GetActorLocation)))
  (Transformation|SetActorLocation (- _output_get (Variables|Default|GetSubtraction)) false false)
  (CallFunction|Spawn))