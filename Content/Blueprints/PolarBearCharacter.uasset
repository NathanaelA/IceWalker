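; Polar bear player character that hops one tile at a time across a board of cubes, logs and water.
; Timelines lerp each move; line traces detect blocked tiles or falls ahead and trigger the landed tile's stepped-on logic.
; Death sinks the bear, restarts the level's ice through GamemodeForNow and replays a rising spawn at the Start checkpoint.
; Delay-driven recursive events toggle step meshes for walking and drive sinking.
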(event Custom|Animate
  (Utilities|FlowControl|Delay 0.1)
  (if (and (Variables|Default|GetAnimateThis) (Variables|Default|GetMoving))
    (Rendering|SetVisibility (Variables|Default|GetStep2) false false)
    (Rendering|SetVisibility (Variables|Default|GetStep4) false false)
    (Rendering|SetVisibility (Variables|Default|GetStep1&3) false false)
    (bind _result (Math|Integer|IncrementInt (Variables|Default|GetAnimateStep))
      (:%20%20
        (switch int _result
          (:Default
            _)
          (:0
            _)
          (:1
            (Rendering|SetVisibility (Variables|Default|GetStep1&3) true false :!label _label))
          (:2
            (Rendering|SetVisibility (Variables|Default|GetStep2) true false))
          (:3
            (goto _label))
          (:4
            (Rendering|SetVisibility (Variables|Default|GetStep4) true false)
            (Variables|Default|SetAnimateStep 0)))
        (CallFunction|Animate)))
    (else
      (Rendering|SetVisibility (Variables|Default|GetStep2) false false)
      (Rendering|SetVisibility (Variables|Default|GetStep4) false false)
      (Rendering|SetVisibility (Variables|Default|GetStep1&3) true false)
      (CallFunction|Animate))))

(event Custom|MoveLeft
  ;[1 1 1] Move Left
  ;;[1 1 1] Player cannot move Left/Right when on a log
  (Utilities|IsValid (Variables|Default|GetLog)
    (:Is%20Not%20Valid
      (bind _continue (CallFunction|SetUpMoving))
      (if _continue
        (Transformation|SetActorTransform (Math|Transform|MakeTransform (Transformation|GetActorLocation) "0.000000,-90.000000,0.000000" "1,1,1"))
        (Variables|Default|SetFacing "NewEnumerator2")
        (bind _stopmovement (CallFunction|DealwithBlockMoving))
        (if _stopmovement
          (CallFunction|StopMoving)
          (else
            (bind _alpha (Timeline|LeftMovement PlayFromStart)
              (:Update
                (bind _exitout (CallFunction|Move _alpha "0.000000,-100.000000, 0"))
                (if _exitout
                  (CallFunction|StopMoving)
                  (Timeline|LeftMovement Stop))))))))))

(event Custom|KillMyself
  (params (Falling%20in :type Boolean))
  (bind _returnvalue (Transformation|GetActorLocation))
  (bind _deathspeed (Variables|Default|GetDeathSpeed))
  (bind _returnvalue_2 (- _returnvalue (Math|Vector|MakeVector 0.0 0.0 _deathspeed)))
  ;[1 1 1] Stop player from moving and the bear from walking (animation)
  (Variables|Default|SetAnimateThis false)
  (Variables|Default|SetMoving true)
  (if Falling%20in
    (Variables|Default|SetOld (Transformation|GetActorRotation))
    (switch Utilities|FlowControl|Switch|SwitchonFacing (Variables|Default|GetFacing)
      (:NewEnumerator0
        (Variables|Default|SetGoal "-90.000000, 0, 0")
        (bind _alpha (Timeline|Falling%20Animation PlayFromStart)
          (:Update
            (Transformation|SetActorRotation (Math|Rotator|Lerp(Rotator) (Variables|Default|GetOld) (Variables|Default|GetGoal) _alpha))
            (if (Math|Float|NearlyEqual(Float) _alpha 1.0 0.01)
              (Utilities|FlowControl|Sequence
                (:then_0
                  (Timeline|Falling%20Animation Stop))
                (:then_1
                  (CallFunction|KillMyself false)))))))
      (:NewEnumerator1
        (Variables|Default|SetGoal "-90.000000,-180.000000, 0")
        (Timeline|Falling%20Animation PlayFromStart))
      (:NewEnumerator2
        (Variables|Default|SetGoal "-90.000000,-89.000000, 0")
        (Timeline|Falling%20Animation PlayFromStart))
      (:NewEnumerator3
        (Variables|Default|SetGoal "-90.000000,90.000000, 0")
        (Timeline|Falling%20Animation PlayFromStart)))
    (else
      (Transformation|SetActorLocation _returnvalue_2 false false)
      (if (< (.Z (Math|Vector|BreakVector _returnvalue_2)) -2e+02)
        (Utilities|FlowControl|Delay 2.0)
        (bind _asgamemode_for_now (Utilities|Casting|CastToGamemodeForNow (Game|GetGameMode)))
        (Variables|/Game/Blueprints/GamemodeForNow.GamemodeForNow_C|SetCurrentPosition _asgamemode_for_now (Variables|/Game/Blueprints/GamemodeForNow.GamemodeForNow_C|GetOldPosition _asgamemode_for_now))
        (bind _currentlevel (Default|GetCurrentLevel _asgamemode_for_now))
        (Default|StartLevel _asgamemode_for_now _currentlevel true)
        (CallFunction|Spawn)
        (Utilities|FlowControl|Delay 1.4)
        (Default|ClearBoardTiles _asgamemode_for_now true true true)
        (else
          (Utilities|FlowControl|Delay 0.01)
          (CallFunction|KillMyself false))))))

(event Custom|MoveUp
  ;[1 1 1] Moving Up
  (bind _continue (CallFunction|SetUpMoving))
  (if _continue
    (Transformation|SetActorTransform (Math|Transform|MakeTransform (Transformation|GetActorLocation) "0, 0, 0" "1,1,1"))
    (Variables|Default|SetFacing "NewEnumerator0")
    (bind _stopmovement (CallFunction|DealwithBlockMoving))
    (if _stopmovement
      (CallFunction|StopMoving)
      (else
        (bind _alpha (Timeline|UpMovement PlayFromStart)
          (:Update
            (bind _exitout (CallFunction|Move _alpha "100.000000,0.000000, 0"))
            (if _exitout
              (CallFunction|StopMoving)
              (Timeline|UpMovement Stop))))))
    (else
      (CallFunction|StopMoving))))

(event Custom|MoveRight
  ;[1 1 1] Moving Right
  ;;[1 1 1] Player Cannot move left/right if on log
  (Utilities|IsValid (Variables|Default|GetLog)
    (:Is%20Not%20Valid
      (bind _continue (CallFunction|SetUpMoving))
      (if _continue
        (Transformation|SetActorTransform (Math|Transform|MakeTransform (Transformation|GetActorLocation) "0.000000,90.000000,0.000000" "1,1,1"))
        (Variables|Default|SetFacing "NewEnumerator3")
        (bind _stopmovement (CallFunction|DealwithBlockMoving))
        (if _stopmovement
          (CallFunction|StopMoving)
          (else
            (bind _alpha (Timeline|RightMovemnet PlayFromStart)
              (:Update
                (bind _exitout (CallFunction|Move _alpha "0.000000,100.000000, 0"))
                (if _exitout
                  (CallFunction|StopMoving)
                  (Timeline|RightMovemnet Stop))))))))))

(event Custom|MoveDown
  ;[1 1 1] Move Down
  (bind _continue (CallFunction|SetUpMoving))
  (if _continue
    (Transformation|SetActorTransform (Math|Transform|MakeTransform (Transformation|GetActorLocation) "0.000000,180.000000,0.000000" "1,1,1"))
    (Variables|Default|SetFacing "NewEnumerator1")
    (bind _stopmovement (CallFunction|DealwithBlockMoving))
    (if _stopmovement
      (CallFunction|StopMoving)
      (else
        (bind _alpha (Timeline|DownMovement PlayFromStart)
          (:Update
            (bind _exitout (CallFunction|Move _alpha "-100.000000, 0, 0"))
            (if _exitout
              (CallFunction|StopMoving)
              (Timeline|DownMovement Stop))))))))

(event Custom|Spawn
  (bind _returnvalue (Transformation|GetActorRotation))
  (bind _returnvalue_2 (Transformation|GetActorLocation))
  (bind _returnvalue_3 (Transformation|GetActorRotation))
  (bind _z (Math|Vector|BreakVector _returnvalue_2))
  (bind _returnvalue_4 (< -62.0 _z))
  ;[1 1 1 1 68] Serious Spaghettii Code....
  ;
  ; Animation of bear spawning...
  (if (< (Variables|Default|GetTimeAttemptedToSpawn) 10)
    (Variables|Default|SetMoving true)
    (Variables|Default|SetAnimateThis false)
    (Utilities|IsValid (Variables|Default|GetCheckpoint)
      (:Is%20Valid
        (Variables|Default|SetTimeAttemptedToSpawn 0)
        (Transformation|SetActorTransform (Math|Transform|MakeTransform (- (Transformation|GetActorLocation (Variables|Default|GetCheckpoint)) "100.000000, 0, 0") "90.000000, 0, 0" "1,1,1"))
        (Variables|Default|SetVectorAddition (Math|Vector|MakeVector 0.0 0.0 (Variables|Default|GetSpawnSpeed)))
        (Transformation|SetActorLocation (+ (Transformation|GetActorLocation) (Variables|Default|GetVectorAddition)) false false :!label _label)
        (if (and (> (.Z (Math|Vector|BreakVector (+ (Transformation|GetActorLocation) (Variables|Default|GetVectorAddition)))) -9e+01) (not (Math|Float|NearlyEqual(Float) (.pitch _returnvalue) 0.0 0.01))) :!label _label_2
          (Transformation|SetActorRotation (Math|Rotator|MakeRotator (.roll _returnvalue_3) (- (.pitch _returnvalue) (Variables|Default|GetSpawnSpeed)) (.yaw _returnvalue_3)))
          (Utilities|FlowControl|Delay 0.01 :!label _label_3)
          (if _returnvalue_4
            (Variables|Default|SetVectorAddition (Math|Vector|MakeVector (Variables|Default|GetSpawnSpeed) 0.0 0.0))
            (if (<= (.X (Math|Vector|BreakVector (Transformation|GetActorLocation (Variables|Default|GetCheckpoint)))) (.X (Math|Vector|BreakVector (Transformation|GetActorLocation))))
              (goto _label_2)
              (else
                (goto _label)))
            (else
              (goto _label)))
          (elif (Class|KismetMathLibrary|XORBoolean _returnvalue_4 (and (> (.Z (Math|Vector|BreakVector (+ (Transformation|GetActorLocation) (Variables|Default|GetVectorAddition)))) -9e+01) (not (Math|Float|NearlyEqual(Float) (.pitch _returnvalue) 0.0 0.01))))
            (if (<= (.X (Math|Vector|BreakVector (Transformation|GetActorLocation (Variables|Default|GetCheckpoint)))) (.X (Math|Vector|BreakVector (Transformation|GetActorLocation))))
              (Variables|Default|SetMoving false)
              (Variables|Default|SetAnimateThis true)
              (else
                (goto _label_3)))
            (else
              (goto _label_3)))))
      (:Is%20Not%20Valid
        (Math|Integer|IncrementInt (Variables|Default|GetTimeAttemptedToSpawn)
          (:%20%20
            (bind _outactors (Actor|GetAllActorsOfClass "/Game/Blueprints/Start.Start_C"))
            (bind _array_element (Utilities|Array|ForEachLoopwithBreak _outactors :!label _label_4)
              (:LoopBody
                (Variables|Default|SetCheckpoint _array_element)
                (goto _label_4 Break))
              (:Completed
                (if (> 5 (Variables|Default|GetTimeAttemptedToSpawn))
                  (Utilities|FlowControl|Delay 0.1)
                  (CallFunction|Spawn)
                  (else
                    (CallFunction|Spawn)))))))))))

(fn ConstructionScript
  (Rendering|SetVisibility (Variables|Default|GetStep2) false false)
  (Rendering|SetVisibility (Variables|Default|GetStep4) false false)
  (CallFunction|Spawn))

(fn CheckBlockUnderMe
  (bind _step1_3 (Variables|Default|GetStep1&3))
  (bind _returnvalue (Transformation|GetWorldLocation _step1_3))
  (bind (_outhit _returnvalue_2) (Collision|LineTraceByChannel _returnvalue (- _returnvalue "0, 0,200.000000") "TraceTypeQuery1" false 0 "None"))
  (if _returnvalue_2
    (Variables|Default|SetOldBlock (.HitActor (Collision|BreakHitResult _outhit)))
    (return)))

(fn CheckStepped
  (bind _returnvalue (Transformation|GetActorLocation))
  (if (Utilities|IsValid (Variables|Default|GetLog))
    (Variables|/Game/Blueprints/Log.Log_C|SetPlayerOn (Variables|Default|GetLog) false)
    (Variables|Default|SetLog (LocalVariables|GetNullValue)))
  (bind (_outhit _returnvalue_2) (Collision|LineTraceByChannel _returnvalue (- _returnvalue "0, 0,200.000000") "TraceTypeQuery1" false 0 "None"))
  (if _returnvalue_2
    (Utilities|Casting|CastToWater (.HitActor (Collision|BreakHitResult _outhit))
      (:then
        (CallFunction|KillMyself false :!label _label))
      (:CastFailed
        (bind _asend (Utilities|Casting|CastToEnd (.HitActor (Collision|BreakHitResult _outhit)))
          (:then
            (Default|Steppedon _asend))
          (:CastFailed
            (bind _aslog (Utilities|Casting|CastToLog (.HitActor (Collision|BreakHitResult _outhit)))
              (:then
                (Default|Steppedon _aslog)
                (Variables|Default|SetLog _aslog))
              (:CastFailed
                (bind _asstart (Utilities|Casting|CastToStart (.HitActor (Collision|BreakHitResult _outhit)))
                  (:then
                    (Default|Steppedon _asstart self)
                    (Variables|Default|SetCheckpoint _asstart))
                  (:CastFailed
                    (bind _asbase_cube (Utilities|Casting|CastToBaseCube (.HitActor (Collision|BreakHitResult _outhit))))
                    (bind _killme (Default|Steppedon _asbase_cube))
                    (if _killme
                      (CallFunction|KillMyself false))))))))))
    (else
      (goto _label))))

(fn SetUpMoving
  (if (Variables|Default|GetMoving)
    (return false)
    (else
      (Variables|Default|SetAnimateThis true)
      (Variables|Default|SetMoving true)
      (Variables|Default|SetRan false)
      (CallFunction|CheckBlockUnderMe)
      (Variables|Default|SetOldLocation (Transformation|GetActorLocation))
      (return true))))

(fn Move
  (params (Alpha :type Float%20%28single-precision%29) (Direction :type Vector))
  (bind _oldlocation (Variables|Default|GetOldLocation))
  (Transformation|SetActorTransform (Math|Transform|MakeTransform (Math|Vector|Lerp(Vector) _oldlocation (+ Direction _oldlocation) Alpha) (Transformation|GetActorRotation) "1,1,1"))
  (Utilities|FlowControl|Sequence
    (:then_0
      (if (and (not (Variables|Default|GetRan)) (> Alpha 0.7))
        (Variables|Default|SetRan true)
        (bind _ascube (Utilities|Casting|CastToCube (Variables|Default|GetOldBlock)))
        (Default|AfterSteppedon _ascube)))
    (:then_1
      (return (== Alpha 1.0)))))

(fn StopMoving
  (Variables|Default|SetOldLocation "0, 0, 0")
  (Variables|Default|SetMoving false)
  (CallFunction|CheckStepped))

(fn GetBlockinFrontOfMe
  (bind _returnvalue (Transformation|GetActorLocation))
  (switch Utilities|FlowControl|Switch|SwitchonFacing (Variables|Default|GetFacing)
    (:NewEnumerator0
      (LocalVariables|SetTop (+ _returnvalue "100.000000,0.000000,200.000000")))
    (:NewEnumerator1
      (LocalVariables|SetTop (- _returnvalue "100.000000, 0,-200.000000")))
    (:NewEnumerator2
      (LocalVariables|SetTop (- _returnvalue "0,100.000000,-200.000000")))
    (:NewEnumerator3
      (LocalVariables|SetTop (+ _returnvalue "0.000000,100.000000,200.000000"))))
  (bind (_outhit _returnvalue_2) (Collision|LineTraceByChannel (LocalVariables|GetTop) (- (LocalVariables|GetTop) "0, 0,800.000000") "TraceTypeQuery1" false 0 "Persistent" true "(R=0.202022,G=0.000000,B=1.000000,A=1.000000)"))
  (if (!= (Utilities|GetClass (.HitActor (Collision|BreakHitResult _outhit))) "/Game/Blueprints/Start.Start_C")
    (if (== (Utilities|GetClass (Variables|Default|GetCheckpoint)) "/Game/Blueprints/End.End_C")
      (bind (_outactor _returnvalue_3) (CallFunction|GetLoginFrontOfMe (LocalVariables|GetTop)))
      (return _outactor _returnvalue_3)
      (else
        _)))
  (return (.HitActor (Collision|BreakHitResult _outhit)) _returnvalue_2))

(fn DealwithBlockMoving
  (bind (_outactor _foundblock) (CallFunction|GetBlockinFrontOfMe))
  (if _foundblock
    (bind _asbase_cube (Utilities|Casting|CastToBaseCube _outactor)
      (:then
        (if (Variables|/Game/Blueprints/BaseCube.BaseCube_C|GethasItem _asbase_cube)
          (return true)
          (else
            _)))
      (:CastFailed
        _))
    (Utilities|Casting|CastToWater _outactor
      (:then
        _)
      (:CastFailed
        (return false))))
  (CallFunction|KillMyself true)
  (return false))

(fn GetLoginFrontOfMe
  (params (Top :type Vector))
  (bind _returnvalue (+ Top "0.000000,-100.000000,-20.000000"))
  (bind _returnvalue_2 (+ Top "0.000000,100.000000,0.000000"))
  (bind (_outhit _returnvalue_3) (Collision|LineTraceByChannel (Math|Vector|MakeVector (.x _returnvalue_2) (.y _returnvalue_2) -6e+01) (Math|Vector|MakeVector (.x _returnvalue) (.y _returnvalue) -9e+01) "TraceTypeQuery1" false 0 "None" true "(R=1.000000,G=0.214236,B=0.000000,A=1.000000)" "(R=0.000000,G=1.000000,B=0.000000,A=1.000000)" 1e+01))
  (return (.HitActor (Collision|BreakHitResult _outhit)) _returnvalue_3))