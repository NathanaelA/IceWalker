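; Start is an actor Blueprint for a block that can be stepped on a limited number of times before it disappears.
; SteppedOn decrements Steps and destroys the actor when the count runs out.
; Otherwise it sets the Cube material from the GamemodeForNow Materials array, indexed by the remaining steps.
; The event graph and construction script are empty, and nothing in the file calls SteppedOn.
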(event EventBeginPlay)

(event Collision|EventActorBeginOverlap
  (params (OtherActor :type Actor%20Object%20Reference)))

(event EventTick
  (params (DeltaSeconds :type Float%20%28single-precision%29)))

(fn ConstructionScript)

(fn Steppedon
  (bind _result (Math|Integer|DecrementInt (Variables|Default|GetSteps))
    (:%20%20
      (if (<= _result 0)
        (Actor|DestroyActor)
        (else
          (bind _asgamemode_for_now (Utilities|Casting|CastToGamemodeForNow (Game|GetGameMode)))
          (Rendering|Material|SetMaterial (Variables|Default|GetCube) 0 (Utilities|Array|Get(acopy) (Variables|/Game/Blueprints/GamemodeForNow.GamemodeForNow_C|GetMaterials _asgamemode_for_now) (Variables|Default|GetSteps))))))))